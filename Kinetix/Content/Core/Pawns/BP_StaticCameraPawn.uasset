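; BP_StaticCameraPawn is a camera pawn that tracks a named bone on another pawn's skeletal mesh from a side-on view.
; On BeginPlay, macros find the mesh, validate the bone name and index with on-screen errors, and record the initial camera-to-bone distance before enabling Tick.
; Each Tick places the pawn at that distance along the bone's right vector, facing back toward the bone.
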(event `self.ReceiveBeginPlay`
  (bind _pawntofollow (`self.PawnToFollow`)
    (:`then`
      (bind _output_get (set `self.SkeletalMeshRef` (`self.GetComponentByClass` _pawntofollow "/Script/Engine.SkeletalMeshComponent")))
      (`/Engine/EditorBlueprintResources/StandardMacros.IsValid` _output_get
        (:`Is Valid`
          (if (not (`KismetStringLibrary.IsEmpty` (`KismetStringLibrary.Conv_NameToString` (`self.BoneToFollow`))))
            (bind _output_get_2 (set `self.BoneIndexToFollow` (`SkinnedMeshComponent.GetBoneIndex` (`self.SkeletalMeshRef`) (`self.BoneToFollow`))))
            (if (>= _output_get_2 0)
              (set `self.DistanceFromPawn` (`KismetMathLibrary.Vector_Distance` (`SceneComponent.GetSocketLocation` (`self.SkeletalMeshRef`) (`self.BoneToFollow`)) (`self.K2_GetActorLocation`)))
              (`self.SetActorTickEnabled` true)
              (else
                (`KismetSystemLibrary.PrintString` (`KismetStringLibrary.Concat_StrStr` "ERROR: No bone " (`KismetStringLibrary.Conv_NameToString` (`self.BoneToFollow`)) " on " (`KismetSystemLibrary.GetObjectName` (`self.PawnToFollow`))) true true (struct :`R` 1.0 :`A` 1.0) 10.0)))
            (else
              (`KismetSystemLibrary.PrintString` (`KismetStringLibrary.Concat_StrStr` "ERROR: No bone name setup for " (`KismetSystemLibrary.GetObjectName` (`self.PawnToFollow`))) true true (struct :`R` 1.0 :`A` 1.0) 10.0))))
        (:`Is Not Valid`
          (`KismetSystemLibrary.PrintString` (`KismetStringLibrary.Concat_StrStr` "ERROR: No skeletal mesh found on " (`KismetSystemLibrary.GetObjectName` (`self.PawnToFollow`))) true true (struct :`R` 1.0 :`A` 1.0) 10.0))))
    (:`else`)))

(event `self.ReceiveTick`
  (params (DeltaSeconds :type "Float (single-precision)"))
  (bind _skeletalmeshref (`self.SkeletalMeshRef`))
  (bind _bonetofollow (`self.BoneToFollow`))
  (bind _returnvalue (`KismetMathLibrary.GetRightVector` (`SceneComponent.GetSocketRotation` _skeletalmeshref _bonetofollow)))
  (`self.K2_SetActorLocationAndRotation` (+ (`SceneComponent.GetSocketLocation` _skeletalmeshref _bonetofollow) (* _returnvalue (`self.DistanceFromPawn`))) (`KismetMathLibrary.MakeRotFromX` (`KismetMathLibrary.NegateVector` _returnvalue))))

(fn `UserConstructionScript`)
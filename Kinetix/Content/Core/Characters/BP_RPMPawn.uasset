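; BP_RPMPawn is a pawn that loads a Ready Player Me avatar at runtime.
; On BeginPlay it hands its target skeletal mesh to the ReadyPlayerMe component and starts the avatar load.
; On success, the Kinetix component checks the anim instance to notify and an avatar-loaded event is called; on failure, the error message is printed.
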(event `self.ReceiveBeginPlay`
  (set `ReadyPlayerMeComponent.SkeletalMeshComponent` (`self.SkeletalMeshTarget`) (`self.ReadyPlayerMe`))
  (`ReadyPlayerMeComponent.LoadAvatar` (`self.ReadyPlayerMe`) (delegate `OnAvatarLoaded`) (delegate `OnAvatarLoadFailed`)))

(event `OnAvatarLoaded`
  (`KinetixCharacterComponent.CheckAnimInstanceToNotify` (`self.KinetixComponent`) self)
  (`self.AvatarLoadedEvent`))

(event `OnAvatarLoadFailed`
  (params (ErrorMessage :type String))
  (`KismetSystemLibrary.PrintString` ErrorMessage))

(fn `UserConstructionScript`)
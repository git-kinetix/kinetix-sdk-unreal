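; Functional test for the Kinetix SDK that covers core setup, account connection and emote playback on a target skeletal mesh.
; StartTest validates the config, then callbacks chain through anim instance registration, account connection, metadata fetch and animation load, using hardcoded IDs.
; The emote plays, then reloads and replays, with fixed delays before the test succeeds; handled failures end it early.
; RemapCurve strips the "mixamorig:" prefix from curve names.
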(event `self.ReceiveBeginPlay`)

(event `self.ReceiveStartTest`
  (bind (_outcoreconfiguration_benableanalytics _outcoreconfiguration_bshowlogs _outcoreconfiguration_cachedemotes _outcoreconfiguration_virtualworld) (break `KinetixCoreConfiguration` (`KinetixDeveloperSettings.GetCoreConfiguration`)))
  (`KinetixCoreSubsystem.RegisterOrCallOnInitialized` (subsystem `KinetixCoreSubsystem`) (delegate `OnKinetixCoreInitialized`))
  (if (not (`KismetStringLibrary.IsEmpty` _outcoreconfiguration_virtualworld))
    (`self.LogMessage` "Core Configuration valid")
    (bind _returnvalue (`KinetixCoreSubsystem.Setup` (subsystem `KinetixCoreSubsystem`) (`KinetixDeveloperSettings.GetCoreConfiguration`)))
    (if _returnvalue
      (`self.LogMessage` "Kinetix Core asked for initialization")
      (else
        (`self.FinishTest` "Failed" "Failed to initialize core")))
    (else
      (`self.FinishTest` "Error" "Core Configuration is invalid"))))

(event `OnKinetixCoreInitialized`
  (bind _kinetixaccount (`KinetixCoreSubsystem.KinetixAccount` (subsystem `KinetixCoreSubsystem`)))
  (`self.LogMessage` "Kinetix Core Initialized successfully")
  (bind _outguid (`KinetixAnimation.RegisterAvatarAnimInstance` (`KinetixCoreSubsystem.KinetixAnimation` (subsystem `KinetixCoreSubsystem`)) (`SkeletalMeshComponent.GetAnimInstance` (`/Game/Overdare/BP_Overdare.SkeletalMesh` (`self.Target`))) "bdb51e82-a97c-4bce-a6e0-64c34d52be18"))
  (set `self.New Anim Instance Guid` _outguid)
  (add `KinetixAccount.OnConnectedAccount` _kinetixaccount (delegate `OnAccountConnected`))
  (`KinetixAccount.ConnectAccount` _kinetixaccount "Alex"))

(event `OnAccountConnected`
  (`self.LogMessage` "Kinetix account connected successfully")
  (bind _output_get (set `self.EmoteToPlay` (`KinetixDataBlueprintFunctionLibrary.GetAnimationIDFromString` "5cd51ab4-2a3b-43a3-b332-ea8dc75d8d93")))
  (`KinetixMetadata.GetAnimationMetadataByAnimationID` (`KinetixCoreSubsystem.KinetixMetadata` (subsystem `KinetixCoreSubsystem`)) _output_get (delegate `OnMetadataAvailable`)))

(event `OnMetadataAvailable`
  (params (bSuccess :type Boolean) (AnimationData :type "AnimationMetadata Structure (by ref)"))
  (bind _kinetixanimation (`KinetixCoreSubsystem.KinetixAnimation` (subsystem `KinetixCoreSubsystem`)))
  (if bSuccess
    (`self.LogMessage` "Animation metadatas available")
    (`KinetixAnimation.SetReferenceSkeleton` _kinetixanimation (`SkeletalMeshComponent.GetSkeletalMeshAsset` (`/Game/Overdare/BP_Overdare.SkeletalMesh` (`self.Target`))))
    (`KinetixAnimation.SetCurveRemapper` _kinetixanimation (`|CreateDelegate` :!event `RemapCurve`))
    (`KinetixAnimation.LoadLocalPlayerAnimation` _kinetixanimation (`.Id` (break `AnimationMetadata` AnimationData)) "bdb51e82-a97c-4bce-a6e0-64c34d52be18" (delegate `OnAnimationLoaded`))
    (else
      (`self.FinishTest` "Failed" "Failed to get metadatas"))))

(event `OnAnimationLoaded`
  (params (Success :type Boolean))
  (if Success
    (`KinetixAnimation.PlayAnimationOnAvatar` (`KinetixCoreSubsystem.KinetixAnimation` (subsystem `KinetixCoreSubsystem`)) (`self.New Anim Instance Guid`) (`self.EmoteToPlay`))
    (`self.LogMessage` "Waiting for animation to finish...")
    (`KismetSystemLibrary.Delay` 5.0)
    (`KinetixAnimation.LoadLocalPlayerAnimation` (`KinetixCoreSubsystem.KinetixAnimation` (subsystem `KinetixCoreSubsystem`)) (`self.EmoteToPlay`) "bdb51e82-a97c-4bce-a6e0-64c34d52be18" (delegate `OnAnimationReloaded`))
    (else
      (`self.FinishTest` "Failed" "Failed to load animation "))))

(event `OnAnimationReloaded`
  (params (Success :type Boolean))
  (if Success
    (`KinetixAnimation.PlayAnimationOnAvatar` (`KinetixCoreSubsystem.KinetixAnimation` (subsystem `KinetixCoreSubsystem`)) (`self.New Anim Instance Guid`) (`self.EmoteToPlay`))
    (`self.LogMessage` "Waiting for animation to finish...")
    (`KismetSystemLibrary.Delay` 5.0)
    (`self.FinishTest` "Succeeded" "Test failed successfully")
    (else
      (`self.FinishTest` "Failed" "Failed to reload animation "))))

(fn `RemapCurve`
  (params (NodeIndex :type Integer) (CurveName :type String) (Path :type String) (Context :type "Object Object Reference"))
  (returns (ReturnValue :type String))
  (return (`KismetStringLibrary.Replace` CurveName "mixamorig:")))

(fn `UserConstructionScript`)
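; Player controller for Kinetix that toggles the Kinetix emote UI on and off.
; BeginPlay creates one CAW_KinetixGenericBase widget and keeps it for reuse.
; The IA_ShowKinetixUI input and the ToggleEmoteWheel event share one toggle path with a debug print, branching on the widget's activated state.
; Opening adds it to the viewport with focused UI-only input; closing deactivates and removes it, then sets Game and UI input.
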(event `self.ReceiveBeginPlay`
  (bind _returnvalue (`|CreateWidget` "/KinetixUI/Kinetix/CAW_KinetixGenericBase.CAW_KinetixGenericBase_C" self))
  (set `self.KinetixUIRef` _returnvalue))

(event `EnhancedInput|/KinetixUI/Inputs/IA_ShowKinetixUI`
  (params (ActionValue :type Boolean) (ElapsedSeconds :type "Float (double-precision)") (TriggeredSeconds :type "Float (double-precision)") (InputAction :type "InputAction Object Reference" :default "/KinetixUI/Inputs/IA_ShowKinetixUI.IA_ShowKinetixUI"))
  (:`Completed`
    (`KismetSystemLibrary.PrintString` "KinetixUI has been asked !" true true (struct :`G` 1.0 :`A` 1.0) 5.0 :!label _label)
    (bind _kinetixuiref (`self.KinetixUIRef`)
      (:`then`
        (if (`CommonActivatableWidget.IsActivated` _kinetixuiref)
          (`CommonActivatableWidget.DeactivateWidget` _kinetixuiref)
          (`Widget.RemoveFromParent` _kinetixuiref)
          (`WidgetBlueprintLibrary.SetInputMode_GameAndUIEx` self null "DoNotLock" true true)
          (else
            (`UserWidget.AddToViewport` _kinetixuiref 0)
            (`WidgetBlueprintLibrary.SetInputMode_UIOnlyEx` self (`CommonActivatableWidget.GetDesiredFocusTarget` _kinetixuiref) "DoNotLock" true))))
      (:`else`))))

(event `ToggleEmoteWheel`
  (goto _label))

(fn `UserConstructionScript`)
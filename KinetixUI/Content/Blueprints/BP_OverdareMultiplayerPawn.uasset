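; BP_OverdareMultiplayerPawn is a player pawn with a Kinetix character and a spring-arm camera that adapts to the player count.
; When a local controller takes over, it resets control rotation, installs the camera input context and sets a hardcoded avatar ID.
; It binds to the PC_ThirdPersonKinetix player-joined event, scaling the default arm length by the player count.
; Enhanced Input turn and look-up actions drive controller yaw and pitch.
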(event `self.ReceiveBeginPlay`
  (set `self.DefaultArmLength` (`SpringArmComponent.TargetArmLength` (`self.SpringArm`))))

(event `self.ReceiveControllerChanged`
  (params (OldController :type "Controller Object Reference") (NewController :type "Controller Object Reference"))
  (`/Engine/EditorBlueprintResources/StandardMacros.IsValid` NewController
    (:`Is Valid`
      (if (`Controller.IsLocalPlayerController` NewController)
        (`Controller.SetControlRotation` NewController (`KismetMathLibrary.MakeRotator` 0.0 0.0 180.0))
        (bind _aspc_third_person_kinetix (cast `/Game/ThirdPerson/Blueprints/PC_ThirdPersonKinetix` (`self.GetController`)))
        (add `/Game/ThirdPerson/Blueprints/PC_ThirdPersonKinetix.OnPlayerJoined` _aspc_third_person_kinetix (delegate `OnPlayerJoined`))
        (bind _returnvalue (pcsubsystem `EnhancedInputLocalPlayerSubsystem` _aspc_third_person_kinetix))
        (`EnhancedInputSubsystemInterface.ClearAllMappings` _returnvalue)
        (`EnhancedInputSubsystemInterface.AddMappingContext` _returnvalue "/KinetixUI/Inputs/IMC_Camera.IMC_Camera" 0 (struct))
        (`KinetixCharacterComponent.SetAvatarID` (`self.KinetixCharacter`) "ddefa996-06c0-40dc-a9a3-dd2c8e090804")))))

(event `OnPlayerJoined`
  (params (NumPlayers :type Byte))
  (set `SpringArmComponent.TargetArmLength` (* NumPlayers (`self.DefaultArmLength`)) (`self.SpringArm`)))

(event `EnhancedInput|/KinetixUI/Inputs/IA_Turn`
  (params (ActionValue :type "Float (double-precision)") (ElapsedSeconds :type "Float (double-precision)") (TriggeredSeconds :type "Float (double-precision)") (InputAction :type "InputAction Object Reference" :default "/KinetixUI/Inputs/IA_Turn.IA_Turn"))
  (:`Triggered`
    (`self.AddControllerYawInput` ActionValue)))

(event `EnhancedInput|/KinetixUI/Inputs/IA_LookUp`
  (params (ActionValue :type "Float (double-precision)") (ElapsedSeconds :type "Float (double-precision)") (TriggeredSeconds :type "Float (double-precision)") (InputAction :type "InputAction Object Reference" :default "/KinetixUI/Inputs/IA_LookUp.IA_LookUp"))
  (:`Triggered`
    (`self.AddControllerPitchInput` ActionValue)))

(fn `UserConstructionScript`)